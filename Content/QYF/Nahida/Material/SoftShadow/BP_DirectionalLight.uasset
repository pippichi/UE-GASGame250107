(fn `ProjMatrix`
  (returns (X :type "Vector4 Structure") (Y :type "Vector4 Structure") (Z :type "Vector4 Structure") (W :type "Vector4 Structure"))
  (bind _scenecapturecomponent2d (`self.SceneCaptureComponent2D`))
  (bind _returnvalue (- 100000.0 1.0))
  ;[1 1 1] 投影矩阵
  (return (`KismetMathLibrary.MakeVector4` (/ 2.0 (`SceneCaptureComponent2D.OrthoWidth` _scenecapturecomponent2d))) (`KismetMathLibrary.MakeVector4` 0.0 (/ -2.0 (`SceneCaptureComponent2D.OrthoWidth` _scenecapturecomponent2d))) (`KismetMathLibrary.MakeVector4` 0.0 0.0 (/ 1.0 _returnvalue) (/ (* 1.0 -1.0) _returnvalue)) (`KismetMathLibrary.MakeVector4` 0.0 0.0 0.0 1.0)))

(fn `UserConstructionScript`
  (bind (_x _y _z _w) (`self.ViewMatrix`))
  (set `self.ViewXYZW` (`|MakeArray` _x _y _z _w))
  (bind (_x_2 _y_2 _z_2 _w_2) (`self.ProjMatrix`))
  (set `self.ProjXYZW` (`|MakeArray` _x_2 _y_2 _z_2 _w_2)))

(fn `ViewMatrix`
  (returns (X :type "Vector4 Structure") (Y :type "Vector4 Structure") (Z :type "Vector4 Structure") (W :type "Vector4 Structure"))
  (bind _scenecapturecomponent2d (`self.SceneCaptureComponent2D`))
  (bind _returnvalue (`SceneComponent.GetRightVector` _scenecapturecomponent2d))
  (bind _returnvalue_2 (`SceneComponent.GetUpVector` _scenecapturecomponent2d))
  (bind _returnvalue_3 (`SceneComponent.GetForwardVector` _scenecapturecomponent2d))
  (bind _returnvalue_4 (`SceneComponent.K2_GetComponentLocation` _scenecapturecomponent2d))
  ;[1 1 1] 视图矩阵
  (return (`KismetMathLibrary.MakeVector4` (.x _returnvalue) (.x _returnvalue_2) (.x _returnvalue_3)) (`KismetMathLibrary.MakeVector4` (.y _returnvalue) (.y _returnvalue_2) (.y _returnvalue_3)) (`KismetMathLibrary.MakeVector4` (.z _returnvalue) (.z _returnvalue_2) (.z _returnvalue_3)) (`KismetMathLibrary.MakeVector4` (* (`KismetMathLibrary.Dot_VectorVector` _returnvalue _returnvalue_4) -1.0) (* (`KismetMathLibrary.Dot_VectorVector` _returnvalue_2 _returnvalue_4) -1.0) (* (`KismetMathLibrary.Dot_VectorVector` _returnvalue_3 _returnvalue_4) -1.0))))