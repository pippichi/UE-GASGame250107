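; Bronya character actor built from several skeletal mesh parts that follow the main body's pose and feed head orientation to their materials.
; Construction links the parts by leader pose and creates dynamic materials on all but Outline.
; HeadForward and HeadRight vectors, based on normalized head-socket offsets in GetHeadVector, are written to those materials.
; Tick refreshes both vectors on body, hair, lash, eye, mouth and emoji, leaving LashOverlay at construction values.
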(event `self.ReceiveTick`
  (params (DeltaSeconds :type "Float (single-precision)"))
  (`self.UpdateMaterials` (`self.SkeletalMesh`))
  (`self.UpdateMaterials` (`self.Hair`))
  (`self.UpdateMaterials` (`self.Lash`))
  (`self.UpdateMaterials` (`self.Eye`))
  (`self.UpdateMaterials` (`self.Mouth`))
  (`self.UpdateMaterials` (`self.Emoji`)))

(fn `ConstructMaterials`
  (params (SkeletalMesh :type "SkeletalMeshComponent Object Reference"))
  (bind (_headforward _headright) (`self.GetHeadVector`))
  (bind (_headforward_2 _headright_2) (`self.GetHeadVector`))
  (for (_array_element _array_index) (`MeshComponent.GetMaterials` SkeletalMesh)
    (bind _asmaterial_instance_dynamic (cast `MaterialInstanceDynamic` _array_element)
      (:`then`
        (`MaterialInstanceDynamic.SetVectorParameterValue` _asmaterial_instance_dynamic "HeadForward" _headforward_2)
        (`MaterialInstanceDynamic.SetVectorParameterValue` _asmaterial_instance_dynamic "HeadRight" _headright_2))
      (:`CastFailed`
        (bind _returnvalue (`PrimitiveComponent.CreateDynamicMaterialInstance` SkeletalMesh _array_index _array_element "None"))
        (`MaterialInstanceDynamic.SetVectorParameterValue` _returnvalue "HeadForward" _headforward)
        (`MaterialInstanceDynamic.SetVectorParameterValue` _returnvalue "HeadRight" _headright))))
  (return))

(fn `UpdateMaterials`
  (params (SkeletalMesh :type "SkeletalMeshComponent Object Reference"))
  (bind (_headforward _headright) (`self.GetHeadVector`))
  (`MeshComponent.SetVectorParameterValueOnMaterials` SkeletalMesh "HeadForward" (`KismetMathLibrary.Conv_LinearColorToVector` _headforward))
  (`MeshComponent.SetVectorParameterValueOnMaterials` SkeletalMesh "HeadRight" (`KismetMathLibrary.Conv_LinearColorToVector` _headright))
  (return))

(fn `UserConstructionScript`
  (`SkinnedMeshComponent.SetLeaderPoseComponent` (`self.Hair`) (`self.SkeletalMesh`) false false)
  (`SkinnedMeshComponent.SetLeaderPoseComponent` (`self.Lash`) (`self.SkeletalMesh`) false false)
  (`SkinnedMeshComponent.SetLeaderPoseComponent` (`self.Eye`) (`self.SkeletalMesh`) false false)
  (`SkinnedMeshComponent.SetLeaderPoseComponent` (`self.Mouth`) (`self.SkeletalMesh`) false false)
  (`SkinnedMeshComponent.SetLeaderPoseComponent` (`self.Emoji`) (`self.SkeletalMesh`) false false)
  (`SkinnedMeshComponent.SetLeaderPoseComponent` (`self.Outline`) (`self.SkeletalMesh`) false false)
  (`SkinnedMeshComponent.SetLeaderPoseComponent` (`self.LashOverlay`) (`self.SkeletalMesh`) false false)
  (`self.ConstructMaterials` (`self.SkeletalMesh`))
  (`self.ConstructMaterials` (`self.Hair`))
  (`self.ConstructMaterials` (`self.Emoji`))
  (`self.ConstructMaterials` (`self.Mouth`))
  (`self.ConstructMaterials` (`self.Eye`))
  (`self.ConstructMaterials` (`self.Lash`))
  (`self.ConstructMaterials` (`self.LashOverlay`)))