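; Fireball projectile for the Fire Blast ability that flies outward, returns to its ReturnToActor and explodes.
; On the server, two chained timelines lerp it to a forward apex, then back toward that actor's live position.
; Within MinExplodeDistance it calls OnHit, applies radial damage effects to nearby living players except its owner, then destroys itself.
; Knockback points away from the blast with pitch forced to 45 degrees, alongside a death impulse.
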(event `self.StartOutgoingTimeline`
  (bind _array (`|MakeArray` (`self.GetOwner`)))
  (`/Engine/EditorBlueprintResources/ActorMacros.Switch Has Authority`
    (:`Authority`
      ; Store Init And Apex Location
      (set `self.InitLocation` (`self.K2_GetActorLocation`))
      (set `self.ApexLocation` (+ (`self.InitLocation`) (* (`self.GetActorForwardVector`) (`self.TravelDistance`))))
      (bind (_direction _outgoingtrack) (`Timeline|OutgoingTraceLine`)
        (:`Update`
          (`self.K2_SetActorLocation` (`KismetMathLibrary.VLerp` (`self.InitLocation`) (`self.ApexLocation`) _outgoingtrack)))
        (:`Finished`
          (bind (_direction_2 _returningtrack) (`Timeline|ReturningTraceLine`)
            (:`Update`
              (`self.K2_SetActorLocation` (`KismetMathLibrary.VLerp` (`self.ApexLocation`) (`self.K2_GetActorLocation` (`self.ReturnToActor`)) _returningtrack))
              (if (`self.IsCloseEnoughToExplode`)
                (`self.OnHit`)
                (`KismetArrayLibrary.Array_AddUnique` _array self)
                (bind _outoverlappingactors (`AuraAbilitySystemLibrary.GetLivePlayerWithinRadius` self _array (`self.RadialDamageOuterRadius`) (`self.K2_GetActorLocation`)))
                (set `self.OverlappingActors` _outoverlappingactors)
                (`AuraAbilitySystemLibrary.SetIsRadialDamageEffectParam` (`self.ExplosionDamageParams`) true (`self.RadialDamageInnerRadius`) (`self.RadialDamageOuterRadius`) (`self.K2_GetActorLocation`))
                (for _array_element (`self.OverlappingActors`)
                  (`AuraAbilitySystemLibrary.SetTargetEffectParamsASC` (`self.ExplosionDamageParams`) (`AbilitySystemBlueprintLibrary.GetAbilitySystemComponent` _array_element))
                  (set `self.KnockbackDirection` (- (`self.K2_GetActorLocation` _array_element) (`self.K2_GetActorLocation`)))
                  (`AuraAbilitySystemLibrary.SetKnockbackDirection` (`self.ExplosionDamageParams`) (`self.OverrideKnockbackPitch`) (`self.KnockbackMagnitude`))
                  (`AuraAbilitySystemLibrary.SetDeathImpulseDirection` (`self.ExplosionDamageParams`) (`self.KnockbackDirection`) (`self.DeathImpulseMagnitude`))
                  (`AuraAbilitySystemLibrary.ApplyDamageEffect` (`self.ExplosionDamageParams`)))
                (`self.K2_DestroyActor`)))))))))

(fn `IsCloseEnoughToExplode`
  (returns (ReturnValue :type Boolean))
  (return (< (`KismetMathLibrary.VSize` (- (`self.K2_GetActorLocation`) (`self.K2_GetActorLocation` (`self.ReturnToActor`)))) (`self.MinExplodeDistance`))))

(fn `OverrideKnockbackPitch`
  (returns (ReturnValue :type "Vector Structure"))
  (bind (_returnvalue_roll _returnvalue_pitch _returnvalue_yaw) (`KismetMathLibrary.BreakRotator` (`KismetMathLibrary.MakeRotFromX` (`self.KnockbackDirection`))))
  (return (`KismetMathLibrary.GetForwardVector` (`KismetMathLibrary.MakeRotator` _returnvalue_roll 45.0 _returnvalue_yaw))))

(fn `UserConstructionScript`)