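; Enemy melee attack gameplay ability that faces the combat target and plays a random tagged attack montage from the combat interface.
; When the montage's tagged gameplay event fires, it gathers living players within a small sphere at the tagged combat socket and damages non-friendly ones.
; A successful hit triggers a melee impact gameplay cue carrying the montage tag and target, then the ability ends, as it also does when the montage finishes or is interrupted.
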(event `self.K2_ActivateAbility`
  (bind _returnvalue (`self.GetAvatarActorFromActorInfo`))
  (set `self.HasHitAttack` false)
  (bind _returnvalue_2 (message `EnemyInterface.GetCombatTarget` _returnvalue))
  (bind _ascombat_interface (cast `CombatInterface` _returnvalue))
  (bind _output_get (set `self.CombatInterface` _ascombat_interface))
  (`CombatInterface.UpdateFacingTarget` _output_get (`Actor.K2_GetActorLocation` _returnvalue_2))
  (bind _returnvalue_3 (`CombatInterface.GetAttackMontages` (`self.CombatInterface`)))
  (bind _output_get_2 (set `self.TaggedMontage` (`self.GetRandomTaggedMontageFromArray` _returnvalue_3)))
  (bind (_montage _montagetag _sockettag) (break `TaggedMontage` _output_get_2))
  (`/Engine/EditorBlueprintResources/StandardMacros.IsValid` _montage
    (:`Is Valid`
      (`AbilityTask_PlayMontageAndWait.CreatePlayMontageAndWaitProxy` "None" _montage 1.0 "None" false
        (:`then`
          (`AbilityTask_WaitGameplayEvent.WaitGameplayEvent` _montagetag null
            (:`EventReceived`
              (bind _returnvalue_4 (`CombatInterface.GetCombatSocketLocation` (`self.CombatInterface`) _sockettag))
              (bind _output_get_3 (set `self.CombatSocketLocation` _returnvalue_4))
              (bind _outoverlappingactors (`AuraAbilitySystemLibrary.GetLivePlayerWithinRadius` self (`|MakeArray` (`self.GetAvatarActorFromActorInfo`)) 45.0 (`self.CombatSocketLocation`)))
              (for _array_element _outoverlappingactors
                (if (`AuraAbilitySystemLibrary.IsNotFriend` (`self.GetAvatarActorFromActorInfo`) _array_element)
                  (`self.CauseDamage` _array_element)
                  (set `self.HasHitAttack` true)))
              (if (`self.HasHitAttack`)
                (bind _returnvalue_5 (message `EnemyInterface.GetCombatTarget` (`self.GetAvatarActorFromActorInfo`)))
                (`self.K2_ExecuteGameplayCueWithParams` (struct :`TagName` "GameplayCue.MeleeImpact") (`AbilitySystemBlueprintLibrary.MakeGameplayCueParameters` 0.0 0.0 (struct) (struct) (struct) (`BlueprintGameplayTagLibrary.MakeGameplayTagContainerFromTag` (`.MontageTag` (break `TaggedMontage` (`self.TaggedMontage`)))) (struct) (`self.CombatSocketLocation`) (0.0 0.0 0.0) null (`self.GetAvatarActorFromActorInfo`) _returnvalue_5)))
              (`self.K2_EndAbility`))))
        (:`OnCompleted`
          (`self.K2_EndAbility` :!label _label))
        (:`OnInterrupted`
          (goto _label))
        (:`OnCancelled`
          (goto _label))))
    (:`Is Not Valid`
      (`self.K2_EndAbility`))))