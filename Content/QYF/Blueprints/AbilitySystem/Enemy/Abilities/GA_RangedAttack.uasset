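; GA_RangedAttack is an enemy gameplay ability that fires a projectile at the avatar's combat target.
; On activation it turns the avatar toward the target via CombatInterface and plays a random tagged attack montage.
; The montage's gameplay event triggers SpawnProjectile from the tagged socket at the target's current location, with optional pitch override.
; The random pick is called separately for montage, event tag and socket; the ability ends when the montage finishes or aborts.
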(event `self.K2_ActivateAbility`
  (bind _returnvalue (`self.GetAvatarActorFromActorInfo`))
  (bind _returnvalue_2 (message `EnemyInterface.GetCombatTarget` _returnvalue))
  (bind _ascombat_interface (cast `CombatInterface` _returnvalue))
  (bind _output_get (set `self.CombatInterface` _ascombat_interface))
  (`CombatInterface.UpdateFacingTarget` _output_get (`Actor.K2_GetActorLocation` _returnvalue_2))
  (bind _returnvalue_3 (`CombatInterface.GetAttackMontages` (`self.CombatInterface`)))
  (bind (_montage _montagetag _sockettag) (break `TaggedMontage` (`self.GetRandomTaggedMontageFromArray` _returnvalue_3)))
  (`/Engine/EditorBlueprintResources/StandardMacros.IsValid` _montage
    (:`Is Valid`
      (`AbilityTask_PlayMontageAndWait.CreatePlayMontageAndWaitProxy` "None" _montage 1.0 "None" false
        (:`then`
          (`AbilityTask_WaitGameplayEvent.WaitGameplayEvent` _montagetag null true
            (:`EventReceived`
              (bind _returnvalue_4 (message `EnemyInterface.GetCombatTarget` (`self.GetAvatarActorFromActorInfo`)))
              (`self.SpawnProjectile` (`Actor.K2_GetActorLocation` _returnvalue_4) _sockettag (`self.ShouldOverridePitch`) (`self.PitchOverride`)))))
        (:`OnCompleted`
          (`self.K2_EndAbility` :!label _label))
        (:`OnInterrupted`
          (goto _label))
        (:`OnCancelled`
          (goto _label))))
    (:`Is Not Valid`
      (`self.K2_EndAbility`))))